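; BasePath_3x3_bp is a path Blueprint that, on BeginPlay, spawns a 1 m path piece at the transform of a referenced actor.
; Prioritized boolean flags pick the branch: convert, straight (StraightPath_1m_bp) or curved (CurvedPath_1m_bp).
; The convert branch's spawn call shows no class.
; The construction script is empty, and NewFunction_0 only returns a transform built from a zero vector.
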(event EventBeginPlay
  (bind _actorref (Variables|Default|GetActorRef))
  (bind _returnvalue (Transformation|GetWorldTransform _actorref))
  (if (Variables|Default|GetBool_ConvertPath_1m)
    (Game|SpawnActorfromClass "/Game/Root/Blueprints/Path_bp/PathPieces_bp/Convertpath_bp.Convertpath_bp_C" _returnvalue "Undefined" 0 0)
    (elif (Variables|Default|GetBool_StraightPath_1m)
      (Game|SpawnActorfromClass "/Game/Root/Blueprints/Path_bp/PathPieces_bp/StraightPath_1m_bp.StraightPath_1m_bp_C" _returnvalue "Undefined" 0 0)
      (elif (Variables|Default|GetBool_CurvedPath_1m)
        (Game|SpawnActorfromClass "/Game/Root/Blueprints/Path_bp/PathPieces_bp/CurvedPath_1m_bp.CurvedPath_1m_bp_C" _returnvalue "Undefined" 0 0)))))

(fn ConstructionScript)

(fn NewFunction0
  (return (Math|Conversions|ToTransform(Vector) "0.000000, 0, 0")))