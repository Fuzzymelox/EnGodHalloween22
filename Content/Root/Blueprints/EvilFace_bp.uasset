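; EvilFace is a pawn that constantly turns toward and creeps after the first-person player character.
; Each Tick it interpolates from its control rotation toward a look-at rotation, using a fixed delta time rather than the frame's, then applies weak forward movement input.
; The pursuit is unconditional, as the PawnSensing sight event is empty.
; BeginPlay only prints what appears to be a version tag.
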(event OnSeePawn(PawnSensing)
  (params (Pawn :type Pawn%20Object%20Reference)))

(event EventBeginPlay
  (Development|PrintString "EGH2_0.1 "))

(event Collision|EventActorBeginOverlap
  (params (OtherActor :type Actor%20Object%20Reference)))

(event EventTick
  (params (DeltaSeconds :type Float%20%28single-precision%29))
  (bind _self self)
  (bind _asfirst_person_character (Utilities|Casting|CastToFirstPersonCharacter (Game|GetPlayerCharacter 0)))
  (Transformation|SetActorRotation (Math|Interpolation|RInterpTo (Pawn|GetControlRotation _self :!class /Script/Engine.Pawn) (Math|Rotator|FindLookatRotation (Transformation|GetActorLocation _self) (Transformation|GetActorLocation _asfirst_person_character)) 1.0 1.0))
  (Pawn|Input|AddMovementInput (Transformation|GetActorForwardVector _self) 0.1 false))

(fn ConstructionScript)